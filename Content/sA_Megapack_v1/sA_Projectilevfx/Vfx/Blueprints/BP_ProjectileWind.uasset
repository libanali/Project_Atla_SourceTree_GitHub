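; BP_ProjectileWind is a wind projectile that plays an impact effect when it hits an Enemy.
; BeginPlay assigns the configured projectile and hit effect assets to their two effect components.
; A Sphere1 hit on an Enemy deactivates the projectile effect, activates and moves the hit effect to the impact point, disables sphere collision and prints a debug message.
; Other hit actors are ignored, and the graph applies no damage and never destroys the actor.
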(event OnComponentHit(Sphere1)
  (params (HitComponent :type Primitive%20Component%20Object%20Reference) (OtherActor :type Actor%20Object%20Reference) (OtherComp :type Primitive%20Component%20Object%20Reference) (NormalImpulse :type Vector :default "0, 0, 0") (Hit :type Hit%20Result%20Structure%20%28by%20ref%29))
  (bind _hiteffects (Variables|Default|GetHiteffects))
  (Utilities|Casting|CastToEnemy OtherActor)
  (Components|Activation|Deactivate (Variables|Default|GetProjectileEffect))
  (Components|Activation|SetActive _hiteffects true false)
  (Transformation|SetWorldLocation _hiteffects (.Location (Collision|BreakHitResult Hit)) false false)
  (Collision|SetCollisionEnabled (Variables|Default|GetSphere1) "NoCollision")
  (Development|PrintString "Wind Hit!" true true "(R=0.053320,G=1.000000,B=0.000000,A=1.000000)"))

(event EventBeginPlay
  (Class|NiagaraComponent|SetAsset (Variables|Default|GetProjectileEffect) (Variables|Default|GetProjectilefx) true)
  (Class|NiagaraComponent|SetAsset (Variables|Default|GetHiteffects) (Variables|Default|GetHitEffect) true))

(fn ConstructionScript)